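; BP_BrokenDoor is a two-panel sliding lab door driven by overlaps on its Collision component.
; Overlap begin and end toggle Open and Close flags, read by a custom event gated by Door.
; Opening steps Pos to 100, sliding the panels apart along Y via absolute world locations, ignoring DeltaSeconds.
; Closing compares against 100 rather than zero, so it snaps Pos to 100 instead of moving the panels back.
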(event `self.Collision.OnComponentBeginOverlap`
  (params (OverlappedComponent :type "PrimitiveComponent Object Reference") (OtherActor :type "Actor Object Reference") (OtherComp :type "PrimitiveComponent Object Reference") (OtherBodyIndex :type Integer) (bFromSweep :type Boolean) (SweepResult :type "HitResult Structure (by ref)"))
  ;[0 0.3281 0] SecurityBreach0X00CF52
  (set `self.Open` true)
  (set `self.Close` false))

(event `self.Collision.OnComponentEndOverlap`
  (params (OverlappedComponent :type "PrimitiveComponent Object Reference") (OtherActor :type "Actor Object Reference") (OtherComp :type "PrimitiveComponent Object Reference") (OtherBodyIndex :type Integer))
  ;[0 0.3281 0] SecurityBreach0X00CF52
  (set `self.Open` false)
  (set `self.Close` true))

(event `CustomEvent`
  (params (DeltaSeconds :type "Float (single-precision)"))
  (bind _pos (`self.Pos`))
  (bind _pos_2 (`self.Pos`))
  (bind _pos_3 (`self.Pos`))
  ;[0 0.3281 0] SecurityBreach0X00CF52
  (if (`self.Door`)
    (if (`self.Open`)
      (`/Engine/EditorBlueprintResources/StandardMacros.CompareFloat` _pos_3 100.0
        (:`>`
          (set `self.Pos` 100.0 :!label _label)
          (set `self.Open` false))
        (:`==`
          (goto _label))
        (:`<`
          (set `self.Pos` (+ _pos_3 2.0))
          (`SceneComponent.K2_SetWorldLocation` (`self.LabDoor03A`) (+ (`KismetMathLibrary.MakeVector` 0.0 _pos_2) (0.0 95.599998 0.0)) false false :!label _label_2)
          (`SceneComponent.K2_SetWorldLocation` (`self.LabDoor03B`) (+ (`KismetMathLibrary.MakeVector` 0.0 (* _pos_2 -1.0)) (0.0 -95.599998 0.0)) false false)))
      (elif (`self.Close`)
        (`/Engine/EditorBlueprintResources/StandardMacros.CompareFloat` _pos 100.0
          (:`>`
            (set `self.Pos` (- _pos 2.0))
            (goto _label_2))
          (:`==`
            _)
          (:`<`
            _))
        (set `self.Pos` 100.0)
        (set `self.Close` false)))))

(fn `UserConstructionScript`)