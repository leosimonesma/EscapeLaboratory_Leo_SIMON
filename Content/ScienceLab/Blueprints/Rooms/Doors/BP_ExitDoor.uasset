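; Sliding double exit door for the Science Lab, opened by a linked Computer.
; Each Tick while the Computer's OpenDoor0 flag is set, it nudges the two panels in opposite directions along local Y by DoorPosition and reapplies a material to the jamb and panels.
; The graph has no travel limit or frame-time scaling.
; The Open node and the construction script's copy of this logic are unconnected.
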(event `self.ReceiveTick`
  (params (DeltaSeconds :type "Float (single-precision)"))
  (bind _doorposition (`self.DoorPosition`))
  ;[1 1 1] Movement
  (if (`/Game/ScienceLab/SecuritySystem/BP_San1taryComputer.OpenDoor_0` (`self.Computer`))
    (`SceneComponent.K2_AddRelativeLocation` (`self.DoorR`) (`KismetMathLibrary.MakeVector` 0.0 _doorposition) false false)
    (`SceneComponent.K2_AddRelativeLocation` (`self.DoorL`) (`KismetMathLibrary.MakeVector` 0.0 (* _doorposition -1.0)) false false)
    ;[1 1 1] Materail
    (`PrimitiveComponent.SetMaterial` (`self.Doorjamb05`) 0 (`self.Materail1`))
    (`PrimitiveComponent.SetMaterial` (`self.DoorL`) 0 (`self.Materail1`))
    (`PrimitiveComponent.SetMaterial` (`self.DoorR`) 0 (`self.Materail1`))))

(fn `UserConstructionScript`)